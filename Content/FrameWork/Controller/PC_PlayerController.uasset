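; Player controller for a turn-based grid card game, handling the first player's move and activate card actions, plus pause.
; Keys 1 and 2 fire those actions on the player's turn, validated by macros checking selection, card type against cell type, or on-board status.
; Success hides all grid selection decals; failure sends messages through the game mode.
; Helpers toggle card HUD buttons by index and display state changes.
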(event `self.ReceiveBeginPlay`
  (`EnhancedInputSubsystemInterface.AddMappingContext` (subsystem `EnhancedInputLocalPlayerSubsystem`) "/Game/FrameWork/Input/IMC_Framework.IMC_Framework" 0 (struct))
  (bind _outactors (`GameplayStatics.GetAllActorsOfClass` "/Game/FrameWork/Blueprint/Grid/BP_GridCell.BP_GridCell_C"))
  (set `self.Cell Actors` _outactors)
  (bind _asgm_game_mode (cast `/Game/FrameWork/Game/GM_GameMode` (`GameplayStatics.GetGameMode`)))
  (set `self.Game Mode` _asgm_game_mode))

(event `Key|One`
  (params (Key :type "Key Structure"))
  ;[1 1 1] Move Card Event
  (:`Pressed`
    (`self.Move Card Event`)))

(event `Move Card Event`
  ;[1 1 1] Move Card Event
  (bind _asgi_game_instance (cast `/Game/FrameWork/Game/GI_GameInstance` (`GameplayStatics.GetGameInstance`))
    (:`then`
      (if (`/Game/FrameWork/Game/GI_GameInstance.PlayerTurn` _asgi_game_instance)
        (`self.CardCanMoveToBoard` _asgi_game_instance
          (:`Continue`
            (`/Game/FrameWork/Blueprint/Card/BP_CardBase.MoveCardToBoard` (`/Game/FrameWork/Blueprint/Character/BP_PlayerBase.GetPlayerSelectedData` (`/Game/FrameWork/Game/GI_GameInstance.PlayerOne` _asgi_game_instance)))
            (`self.ResetGridSelection`))
          (:`Cancel`
            (`/Game/FrameWork/Game/GM_GameMode.UpdateMessage` (`self.Game Mode`) "Invalid Position" "Card Cannot be placed on that position")))))
    (:`CastFailed`
      (`KismetSystemLibrary.PrintString` "Cast Failed" true true (struct :`R` 0.579167 :`B` 0.021519 :`A` 1.0)))))

(event `EnhancedInput|/Game/FrameWork/Input/Actions/IA_Pause`
  (params (ActionValue :type Boolean) (ElapsedSeconds :type "Float (double-precision)") (TriggeredSeconds :type "Float (double-precision)") (InputAction :type "InputAction Object Reference" :default "/Game/FrameWork/Input/Actions/IA_Pause.IA_Pause"))
  (:`Started`
    (`KismetSystemLibrary.PrintString` "Paused Pressed")
    (`/Game/FrameWork/Game/GM_GameMode.PauseGame` (`self.Game Mode`))))

(event `Key|Two`
  (params (Key :type "Key Structure"))
  ;[1 1 1] Activate Card Event
  (:`Pressed`
    (`self.ActivateCardEvent`)))

(event `ActivateCardEvent`
  ;[1 1 1] Activate Card Event
  (bind _asgi_game_instance (cast `/Game/FrameWork/Game/GI_GameInstance` (`GameplayStatics.GetGameInstance`))
    (:`then`
      (if (`/Game/FrameWork/Game/GI_GameInstance.PlayerTurn` _asgi_game_instance)
        (`self.CardCanBeActivated` _asgi_game_instance
          (:`Continue`
            (`/Game/FrameWork/Data/Interfaces/BPI_CardInterface.ActivateCard` (`.SelectedCard_31_67064620492583AC0F84F5B23818FAB3` (break `/Game/FrameWork/Data/Struct/S_PlayerSession` (`/Game/FrameWork/Data/Functions/BPFL_Game.GetPlayerOneSession` self))))
            (`self.ResetGridSelection`))
          (:`Cancel`
            (`/Game/FrameWork/Game/GM_GameMode.UpdateMessage` (`self.Game Mode`) "Message" "Card Cannot be Activated")))))
    (:`CastFailed`
      (`KismetSystemLibrary.PrintString` "Cast Failed" true true (struct :`R` 0.579167 :`B` 0.021519 :`A` 1.0)))))

(event `EnableButtons`
  (params (index :type Integer))
  ;[0.6958 0.1802 0] Index - 0: Add Card Button, 1: Move Card Button, 2 : Activate Card Button, 3 : Disable all Button
  (bind _ashbp_hud (cast `/Game/FrameWork/UI/HBP_HUD` (`self.GetHUD`)))
  (bind _aswb_card_hud (cast `/Game/FrameWork/UI/Widgets/WB_CardHUD` (`/Game/FrameWork/UI/HBP_HUD.ActiveWidgetRef` _ashbp_hud)))
  (switch `int` index
    (:`Default`
      (`/Game/FrameWork/UI/Widgets/WB_CardHUD.DisableAllButton` _aswb_card_hud))
    (:`0`
      (`/Game/FrameWork/UI/Widgets/WB_CardHUD.EnableAddCardButton` _aswb_card_hud))
    (:`1`
      (`/Game/FrameWork/UI/Widgets/WB_CardHUD.EnableMoveCardButton` _aswb_card_hud))
    (:`2`
      (`/Game/FrameWork/UI/Widgets/WB_CardHUD.EnableActivateButton` _aswb_card_hud))))

(fn `ResetGridSelection`
  (for _array_element (`self.Cell Actors`)
    (`SceneComponent.SetVisibility` (`/Game/FrameWork/Blueprint/Grid/BP_GridCell.SelectionDecal` _array_element) false false)))

(fn `UpdateState`
  (params (PlayerStateEnum :type "/Game/FrameWork/Data/Enum/E_PlayerState Enum" :default "NewEnumerator0"))
  (bind _ashbp_hud (cast `/Game/FrameWork/UI/HBP_HUD` (`self.GetHUD`)))
  (bind _aswb_card_hud (cast `/Game/FrameWork/UI/Widgets/WB_CardHUD` (`/Game/FrameWork/UI/HBP_HUD.ActiveWidgetRef` _ashbp_hud)))
  (bind _output_get (set `self.PlayerStateEnum` PlayerStateEnum))
  (`/Game/FrameWork/UI/Widgets/WB_CardHUD.UpdateMessage` _aswb_card_hud (`KismetTextLibrary.Conv_StringToText` (`|GetEnumeratorNameAsString` _output_get)) ""))

(fn `UserConstructionScript`)