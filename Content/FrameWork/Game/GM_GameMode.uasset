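; Game mode for a card game between the player and an AI, managing setup, match start, turn switching and pause.
; On BeginPlay it caches the game instance and player controller, then resets BP_Player and BP_AI and stores them there as PlayerOne and PlayerTwo.
; StartGame shows the card HUD and spawns cards for both sides with delays.
; Other events push stats and messages to the HUD widget and refresh hand positions.
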(event `self.ReceiveBeginPlay`
  (`|ExecutionSequence`
    (:`then_0`
      (`self.SetupControllerAndInstance`))
    (:`then_1`
      (`self.SetupPlayers`))))

(event `self.ReceiveTick`
  (params (DeltaSeconds :type "Float (single-precision)")))

(event `UpdatePlayerUI`
  (bind _playerone (`/Game/FrameWork/Game/GI_GameInstance.PlayerOne` (`self.Game Instance`)))
  (bind (_cardsondeck _cardsinhand _cardsonboard _unitsonboard) (`/Game/FrameWork/Blueprint/Character/BP_PlayerBase.GetPlayerCardAndUnitInfo` _playerone))
  (bind (_id _name _type _bisplayer _health) (`/Game/FrameWork/Blueprint/Character/BP_PlayerBase.GetPlayerInfo` _playerone))
  ;[0.01247 0.2903 1] UPDATE UI STAT
  (bind _ashbp_hud (cast `/Game/FrameWork/UI/HBP_HUD` (`PlayerController.GetHUD` (`self.Player Controller`))))
  (bind _aswb_card_hud (cast `/Game/FrameWork/UI/Widgets/WB_CardHUD` (`/Game/FrameWork/UI/HBP_HUD.ActiveWidgetRef` _ashbp_hud)))
  (`/Game/FrameWork/UI/Widgets/Stat/WB_Stat.OnHandChanged` (`/Game/FrameWork/UI/Widgets/WB_CardHUD.WB_PlayerStat` _aswb_card_hud) (`KismetTextLibrary.Conv_NameToText` _name) _health _unitsonboard _cardsinhand _cardsondeck _cardsonboard))

(event `StartGame`
  (bind _playertwo (`/Game/FrameWork/Game/GI_GameInstance.PlayerTwo` (`self.Game Instance`)))
  (bind _playerone (`/Game/FrameWork/Game/GI_GameInstance.PlayerOne` (`self.Game Instance`)))
  ;[0.1302 1 0] Start Game and Spawn Cards For Both AI and Player
  (`|ExecutionSequence`
    (:`then_0`
      (bind _ashbp_hud (cast `/Game/FrameWork/UI/HBP_HUD` (`PlayerController.GetHUD` (`self.Player Controller`))))
      (`/Game/FrameWork/UI/HBP_HUD.ShowCardHudMenu` _ashbp_hud))
    (:`then_1`
      (for _ (range 2)
        (`/Game/FrameWork/Blueprint/Character/BP_PlayerBase.SpawnCard` :`self` _playerone)
        (`KismetSystemLibrary.Delay` 5.0))
      (set `/Game/FrameWork/Blueprint/Character/BP_PlayerBase.CurrentState` "NewEnumerator1" _playerone)
      (set `self.bIsPlayerTurn` true))
    (:`then_2`
      (for _ (range 2)
        (`/Game/FrameWork/Blueprint/Character/BP_PlayerBase.SpawnCard` :`self` _playertwo)
        (`KismetSystemLibrary.Delay` 5.0))
      (set `/Game/FrameWork/Blueprint/Character/BP_PlayerBase.CurrentState` "NewEnumerator0" _playertwo))))

(event `UpdateAIStat`
  (bind _playertwo (`/Game/FrameWork/Game/GI_GameInstance.PlayerTwo` (`self.Game Instance`)))
  (bind (_cardsondeck _cardsinhand _cardsonboard _unitsonboard) (`/Game/FrameWork/Blueprint/Character/BP_PlayerBase.GetPlayerCardAndUnitInfo` _playertwo))
  (bind (_id _name _type _bisplayer _health) (`/Game/FrameWork/Blueprint/Character/BP_PlayerBase.GetPlayerInfo` _playertwo))
  ;[0.01247 0.2903 1] UPDATE AI STAT
  (bind _ashbp_hud (cast `/Game/FrameWork/UI/HBP_HUD` (`PlayerController.GetHUD` (`self.Player Controller`))))
  (bind _aswb_card_hud (cast `/Game/FrameWork/UI/Widgets/WB_CardHUD` (`/Game/FrameWork/UI/HBP_HUD.ActiveWidgetRef` _ashbp_hud)))
  (`/Game/FrameWork/UI/Widgets/Stat/WB_Stat.OnHandChanged` (`/Game/FrameWork/UI/Widgets/WB_CardHUD.WB_AiStat` _aswb_card_hud) (`KismetTextLibrary.Conv_NameToText` _name) _health _unitsonboard _cardsinhand _cardsondeck _cardsonboard))

(event `UpdateMessage`
  (params (Title :type Text) (Message :type Text))
  ;[0.01247 0.2903 1] UPDATE UI MESSAGE FROM GAME MODE
  (bind _ashbp_hud (cast `/Game/FrameWork/UI/HBP_HUD` (`PlayerController.GetHUD` (`self.Player Controller`))))
  (bind _aswb_card_hud (cast `/Game/FrameWork/UI/Widgets/WB_CardHUD` (`/Game/FrameWork/UI/HBP_HUD.ActiveWidgetRef` _ashbp_hud)))
  (`/Game/FrameWork/UI/Widgets/WB_CardHUD.UpdateMessage` _aswb_card_hud Title Message))

(event `UpdateCardDecks`
  (bind _game_instance (`self.Game Instance`))
  ;[0.1302 1 0] Update Card Decks in Level
  (`/Game/FrameWork/Blueprint/Character/BP_PlayerBase.UpdateCardPositionOnHand` (`/Game/FrameWork/Game/GI_GameInstance.PlayerOne` _game_instance))
  (`/Game/FrameWork/Blueprint/Character/BP_PlayerBase.UpdateCardPositionOnHand` (`/Game/FrameWork/Game/GI_GameInstance.PlayerTwo` _game_instance)))

(event `SetupPlayerEvent`
  (bind _game_instance (`self.Game Instance`))
  ;[0.5792 0 0.02152] Player Setup
  (bind _asbp_player (cast `/Game/FrameWork/Blueprint/Character/Player/BP_Player` (`GameplayStatics.GetPlayerPawn` 0)))
  (`/Game/FrameWork/Blueprint/Character/BP_PlayerBase.ResetPlayer` _asbp_player)
  (bind _returnvalue (`GameplayStatics.GetActorOfClass` "/Game/FrameWork/Blueprint/Character/AI/BP_AI.BP_AI_C"))
  (`/Game/FrameWork/Blueprint/Character/BP_PlayerBase.ResetPlayer` _returnvalue)
  (set `/Game/FrameWork/Game/GI_GameInstance.PlayerOne` _asbp_player _game_instance)
  (set `/Game/FrameWork/Game/GI_GameInstance.PlayerTwo` _returnvalue _game_instance))

(event `SwitchTurn`
  (if (`self.bIsPlayerTurn`)
    (set `self.bIsPlayerTurn` false)
    (`self.UpdateMessage` "Opponent's Turn")
    (else
      (set `self.bIsPlayerTurn` true)
      (`self.UpdateMessage` "Your Turn"))))

(event `PauseGame`
  ;[0.1302 1 0] Pause Game Logic
  (`GameplayStatics.SetGamePaused` true)
  (bind _ashbp_hud (cast `/Game/FrameWork/UI/HBP_HUD` (`PlayerController.GetHUD` (`self.Player Controller`))))
  (`/Game/FrameWork/UI/HBP_HUD.ShowPauseMenu` _ashbp_hud))

(event `ResumeGame`
  ;[0.1302 1 0] Pause Game Logic
  (`GameplayStatics.SetGamePaused` false)
  (bind _ashbp_hud (cast `/Game/FrameWork/UI/HBP_HUD` (`PlayerController.GetHUD` (`self.Player Controller`))))
  (`/Game/FrameWork/UI/HBP_HUD.ShowCardHudMenu` _ashbp_hud))

(fn `SetupControllerAndInstance`
  (bind _asgi_game_instance (cast `/Game/FrameWork/Game/GI_GameInstance` (`GameplayStatics.GetGameInstance`)))
  (set `self.Game Instance` _asgi_game_instance)
  (bind _aspc_player_controller (cast `/Game/FrameWork/Controller/PC_PlayerController` (`GameplayStatics.GetPlayerController` 0)))
  (set `self.Player Controller` _aspc_player_controller))

(fn `SetupPlayers`
  (bind _game_instance (`self.Game Instance`))
  (bind _asbp_player (cast `/Game/FrameWork/Blueprint/Character/Player/BP_Player` (`GameplayStatics.GetPlayerPawn` 0)))
  (`/Game/FrameWork/Blueprint/Character/BP_PlayerBase.ResetPlayer` _asbp_player)
  (bind _returnvalue (`GameplayStatics.GetActorOfClass` "/Game/FrameWork/Blueprint/Character/AI/BP_AI.BP_AI_C"))
  (`/Game/FrameWork/Blueprint/Character/BP_PlayerBase.ResetPlayer` _returnvalue)
  (set `/Game/FrameWork/Game/GI_GameInstance.PlayerOne` _asbp_player _game_instance)
  (set `/Game/FrameWork/Game/GI_GameInstance.PlayerTwo` _returnvalue _game_instance)
  (`KismetSystemLibrary.PrintString` "Player Set Successfully" true true (struct :`R` 0.130239 :`G` 1.0 :`A` 1.0) 5.0))

(fn `UserConstructionScript`)