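; Grid manager that spawns a grid of BP_GridCell actors from its own location on BeginPlay.
; GenerateGrid spaces cells by TileSize at a set Height, skips the CenterIndex column, passes each cell its indices and binds its cursor-over event; TestEvent only prints "Hover".
; TileToGrid converts indices to world X/Y with an optional half-tile centre offset, mapping Row to X whereas spawning maps column to X.
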(event `self.ReceiveBeginPlay`
  (`self.GenerateGrid`))

(event `TestEvent`
  (params (TouchedActor :type "Actor Object Reference"))
  (`KismetSystemLibrary.PrintString` "Hover"))

(fn `GenerateGrid`
  (bind (_returnvalue_x _returnvalue_y) (`KismetMathLibrary.BreakVector` (`self.K2_GetActorLocation`)))
  (for _index (range (`self.Col`))
    (if (!= _index (`self.CenterIndex`))
      (for _index_2 (range (`self.Row`))
        (bind _returnvalue (`|SpawnActorFromClass` "/Game/FrameWork/Blueprint/Grid/BP_GridCell.BP_GridCell_C" (`KismetMathLibrary.MakeTransform` (`KismetMathLibrary.MakeVector` (+ (`KismetMathLibrary.Conv_IntToDouble` (* _index (`self.Tile Size`))) _returnvalue_x) (+ (`KismetMathLibrary.Conv_IntToDouble` (* _index_2 (`self.Tile Size`))) _returnvalue_y) (`self.Height`))) "AlwaysSpawn" "MultiplyWithRoot" null _index _index_2 null))
        (add `self.OnBeginCursorOver` _returnvalue (`|CreateDelegate` :!event `TestEvent`))))))

(fn `TileToGrid`
  (params (Row :type Integer) (Column :type Integer) (`bCenter?` :type Boolean))
  (returns (`Grid Location X` :type "Float (double-precision)") (`Grid Location Y` :type "Float (double-precision)"))
  (bind (_returnvalue_x _returnvalue_y) (`KismetMathLibrary.BreakVector` (`self.K2_GetActorLocation`)))
  (bind _returnvalue (select `bool` `bCenter?` :`true` (/ (`self.Tile Size`) 2.0)))
  (return (+ (+ (* Row (`self.Tile Size`)) _returnvalue_x) _returnvalue) (+ _returnvalue (+ _returnvalue_y (* Column (`self.Tile Size`))))))

(fn `UserConstructionScript`)