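; BP_GridCell is a clickable board cell that the player picks as the destination for a selected card.
; Hovering outlines it through custom depth stencil, with a different value for player cells.
; Clicking a player cell toggles selection; selecting requires it be unoccupied, resets BP_GridManager's selection, and registers with PlayerOne before showing the decal, enabling controller buttons and messaging through GM_GameMode.
; The construction script orients the spawn arrow by column.
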(event `self.ReceiveBeginPlay`
  (bind _asgm_game_mode (cast `/Game/FrameWork/Game/GM_GameMode` (`GameplayStatics.GetGameMode`)))
  (set `self.GM Game Mode` _asgm_game_mode)
  (`TextRenderComponent.K2_SetText` (`self.TextRender`) (`KismetTextLibrary.Conv_StringToText` (`KismetStringLibrary.Concat_StrStr` "C :" (`KismetStringLibrary.Conv_IntToString` (`self.ColIndex`)) ", R :" (`KismetStringLibrary.Conv_IntToString` (`self.RowIndex`)))))
  (add `self.OnClicked` (delegate `OnClicked_Event`)))

(event `OnClicked_Event` :!signature `self.OnClicked`
  (params (TouchedActor :type "Actor Object Reference") (ButtonPressed :type "Key Structure" :default "None")))

(event `self.TileMesh.OnBeginCursorOver`
  (params (TouchedComponent :type "PrimitiveComponent Object Reference"))
  (bind _tilemesh (`self.TileMesh`))
  (`PrimitiveComponent.SetRenderCustomDepth` _tilemesh true)
  (if (`self.IsPlayerCell`)
    (`PrimitiveComponent.SetCustomDepthStencilValue` _tilemesh 255)
    (else
      (`PrimitiveComponent.SetCustomDepthStencilValue` _tilemesh 200))))

(event `self.TileMesh.OnEndCursorOver`
  (params (TouchedComponent :type "PrimitiveComponent Object Reference"))
  (bind _tilemesh (`self.TileMesh`))
  (`PrimitiveComponent.SetRenderCustomDepth` _tilemesh false)
  (`PrimitiveComponent.SetCustomDepthStencilValue` _tilemesh 3))

(event `self.TileMesh.OnClicked`
  (params (TouchedComponent :type "PrimitiveComponent Object Reference") (ButtonPressed :type "Key Structure"))
  (if (`self.IsPlayerCell`)
    (if (not (`self.bIsSelected`))
      (`self.SelectThisCell`)
      (else
        (`SceneComponent.SetVisibility` (`self.SelectionDecal`) false false)
        (set `self.bIsSelected` false)))))

(event `SelectThisCell`
  (if (not (`self.bISOccupied`))
    (bind _returnvalue (`GameplayStatics.GetActorOfClass` "/Game/FrameWork/Blueprint/Grid/BP_GridManager.BP_GridManager_C"))
    (`/Game/FrameWork/Blueprint/Grid/BP_GridManager.Reset Grid Selection` _returnvalue)
    (bind _asgi_game_instance (cast `/Game/FrameWork/Game/GI_GameInstance` (`GameplayStatics.GetGameInstance`)))
    (bind _success (`/Game/FrameWork/Blueprint/Character/BP_PlayerBase.SetSelectedCell` (`/Game/FrameWork/Game/GI_GameInstance.PlayerOne` _asgi_game_instance) self))
    (if _success
      (`SceneComponent.SetVisibility` (`self.SelectionDecal`) true false)
      (set `self.bIsSelected` true)
      (bind _aspc_player_controller (cast `/Game/FrameWork/Controller/PC_PlayerController` (`GameplayStatics.GetPlayerController` 0)))
      (`/Game/FrameWork/Controller/PC_PlayerController.EnableButtons` _aspc_player_controller 1)
      (`/Game/FrameWork/Game/GM_GameMode.UpdateMessage` (`self.GM Game Mode`) "Info" "Click on Move Button to move card to selected cell")
      (else
        (`/Game/FrameWork/Game/GM_GameMode.UpdateMessage` (`self.GM Game Mode`) "Info" "Card must be selected first")))
    (else
      (`KismetSystemLibrary.PrintString` "This Cell Is Occupied"))))

(fn `SetUpDirection`
  (bind _colindex (`self.ColIndex`))
  (`SceneComponent.K2_SetWorldRotation` (`self.SpawnDirectionArrow`) (`KismetMathLibrary.MakeRotator` 0.0 0.0 (select `bool` (and (>= _colindex 0) (<= _colindex 1)) :`false` -180.0)) false false))

(fn `UserConstructionScript`
  (`self.SetUpDirection`))