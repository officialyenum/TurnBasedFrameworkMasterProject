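; BP_UnitBase is a base unit that resolves combat as a winner-takes-all stat comparison.
; AttackTarget applies its Attack as damage to the Unit or Card argument, chosen by whether Card is valid.
; On damage from another unit, it compares damage against its Attack or Defence by state; the loser enables mesh physics, then is destroyed after a delay.
; Cursor hover prints the unit's name, and leaving removes OutlineMesh.
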(event `self.ReceiveBeginPlay`
  (bind _mesh (`self.Mesh`))
  (add `PrimitiveComponent.OnBeginCursorOver` _mesh (delegate `OnBeginCursorOver_Event`))
  (add `PrimitiveComponent.OnEndCursorOver` _mesh (delegate `OnEndCursorOver_Event`)))

(event `OnBeginCursorOver_Event`
  (params (TouchedComponent :type "PrimitiveComponent Object Reference"))
  (`KismetSystemLibrary.PrintString` (`KismetSystemLibrary.GetDisplayName` self)))

(event `OnEndCursorOver_Event`
  (params (TouchedComponent :type "PrimitiveComponent Object Reference"))
  (bind _outlinemesh (`self.OutlineMesh`))
  (`/Engine/EditorBlueprintResources/StandardMacros.IsValid` _outlinemesh
    (:`Is Valid`
      (`ActorComponent.K2_DestroyComponent` _outlinemesh))))

(event `self.ReceiveAnyDamage`
  (params (Damage :type "Float (single-precision)") (DamageType :type "DamageType Object Reference") (InstigatedBy :type "Controller Object Reference") (DamageCauser :type "Actor Object Reference"))
  (bind (_state _type _unitclass _attack _defence) (break `/Game/FrameWork/Data/Struct/S_Unit` (`self.State`)))
  (bind _asbp_unit_base (cast `/Game/FrameWork/Blueprint/Unit/BP_UnitBase` DamageCauser))
  (switch `/Game/FrameWork/Data/Enum/E_UnitState` _state
    (:`NewEnumerator0`
      (if (> Damage _attack)
        (`KismetSystemLibrary.PrintString` "Defeat" :!label _label)
        (`PrimitiveComponent.SetSimulatePhysics` (`self.Mesh`) true)
        (`KismetSystemLibrary.Delay` 5.0)
        (`self.K2_DestroyActor`)
        (else
          (`PrimitiveComponent.SetSimulatePhysics` (`Character.Mesh` _asbp_unit_base) true :!label _label_2)
          (`KismetSystemLibrary.Delay` 5.0)
          (`self.K2_DestroyActor` _asbp_unit_base))))
    (:`NewEnumerator1`
      (if (> Damage _defence)
        (goto _label)
        (else
          (goto _label_2))))))

(event `AttackTarget`
  (params (Unit :type "/Game/FrameWork/Blueprint/Unit/BP_UnitBase Object Reference") (Card :type "/Game/FrameWork/Blueprint/Card/BP_CardBase Object Reference"))
  (bind (_state _type _unitclass _attack) (break `/Game/FrameWork/Data/Struct/S_Unit` (`self.State`)))
  (`/Engine/EditorBlueprintResources/StandardMacros.IsValid` Card
    (:`Is Valid`
      (`GameplayStatics.ApplyDamage` Unit _attack null self))
    (:`Is Not Valid`
      (`/Engine/EditorBlueprintResources/StandardMacros.IsValid` Unit
        (:`Is Valid`
          (`GameplayStatics.ApplyDamage` Card _attack null self))))))

(fn `UserConstructionScript`)