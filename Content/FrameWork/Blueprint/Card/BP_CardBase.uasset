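; Base card actor for a two-player, turn-based card game against AI, showing its card info on a front widget.
; Hover toggles a custom-depth highlight; clicks select the card in the HUD or flip it when on the board.
; Timelines animate movement to the selected cell and rotations that toggle visibility.
; Activation converts Unit and Monster cards into spawned actors for the active player; Spell and Trap only print and reselect.
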(event `self.ReceiveBeginPlay`
  (`KismetSystemLibrary.DelayUntilNextTick`)
  (`|ExecutionSequence`
    (:`then_0`
      (bind _aswb_card (cast `/Game/FrameWork/UI/Widgets/WB_Card` (`WidgetComponent.GetUserWidgetObject` (`self.FrontWidget`))))
      (set `self.WB Card UI Ref` _aswb_card)
      (bind _asgm_game_mode (cast `/Game/FrameWork/Game/GM_GameMode` (`GameplayStatics.GetGameMode`)))
      (set `self.GM Game Mode` _asgm_game_mode)
      (`self.SetupUIHud`)
      (bind _asgi_game_instance (cast `/Game/FrameWork/Game/GI_GameInstance` (`GameplayStatics.GetGameInstance`)))
      (set `self.Game Instance` _asgi_game_instance))
    (:`then_1`
      (`self.SetupCard` (`self.CardInfo`)))
    (:`then_2`
      (add `self.OnClicked` (delegate `OnClicked_Event`))
      (add `self.OnBeginCursorOver` (delegate `OnBeginCursorOver_Event`))
      (add `self.OnEndCursorOver` (delegate `OnEndCursorOver_Event`)))))

(event `OnBeginCursorOver_Event` :!signature `self.OnBeginCursorOver`
  (params (TouchedActor :type "Actor Object Reference"))
  (`/Game/FrameWork/Data/Interfaces/BPI_CardInterface.HighlightCard`))

(event `OnEndCursorOver_Event` :!signature `self.OnEndCursorOver`
  (params (TouchedActor :type "Actor Object Reference"))
  (`self.UnHighlightCard`))

(event `OnClicked_Event` :!signature `self.OnClicked`
  (params (TouchedActor :type "Actor Object Reference") (ButtonPressed :type "Key Structure" :default "None"))
  (if (`self.bIsOnBoard`)
    (`self.FlipCard`)
    (else
      (`self.ShowSelectedCard`))))

(event `/Game/FrameWork/Data/Interfaces/BPI_CardInterface.SetupCard`
  (params (CardInfo :type "/Game/FrameWork/Data/Struct/S_Card Structure"))
  (bind _wb_card_ui_ref (`self.WB Card UI Ref`))
  (`/Engine/EditorBlueprintResources/StandardMacros.IsValid` _wb_card_ui_ref
    (:`Is Valid`
      (`/Game/FrameWork/UI/Widgets/WB_Card.OnUpdate` _wb_card_ui_ref CardInfo))))

(event `/Game/FrameWork/Data/Interfaces/BPI_CardInterface.ActivateCard`
  (bind _game_instance (`self.Game Instance`))
  (bind (_name _image _info _type _rank _unit _actorclass) (break `/Game/FrameWork/Data/Struct/S_Card` (`self.CardInfo`)))
  (bind _returnvalue (`SceneComponent.K2_GetComponentToWorld` (`self.SpawnDirectionArrow`)))
  (switch `/Game/FrameWork/Data/Enum/E_CardType` _type
    (:`NewEnumerator0`
      (bind _returnvalue_2 (`|SpawnActorFromClass` _actorclass (`KismetMathLibrary.MakeTransform` (.location _returnvalue) (`KismetMathLibrary.MakeRotator` 0.0 0.0 (.yaw (.rotation _returnvalue)))) "Undefined" "MultiplyWithRoot" null (struct) null :!label _label))
      (if (`/Game/FrameWork/Game/GM_GameMode.bIsPlayerTurn` (`self.GM Game Mode`))
        (`/Game/FrameWork/Blueprint/Character/BP_PlayerBase.ConvertCardToUnit` (`/Game/FrameWork/Game/GI_GameInstance.PlayerOne` _game_instance) self _returnvalue_2)
        (`self.K2_DestroyActor`)
        (else
          (`/Game/FrameWork/Blueprint/Character/BP_PlayerBase.ConvertCardToUnit` (`/Game/FrameWork/Game/GI_GameInstance.PlayerTwo` _game_instance) self _returnvalue_2)
          (`KismetSystemLibrary.PrintString` "AI Spawned Unit" true true (struct :`R` 0.579167 :`B` 0.021519 :`A` 1.0) 5.0)
          (`self.K2_DestroyActor`))))
    (:`NewEnumerator1`
      (goto _label))
    (:`NewEnumerator2`
      (`KismetSystemLibrary.PrintString` "Spell Applied")
      (`self.ShowSelectedCard`))
    (:`NewEnumerator3`
      (`KismetSystemLibrary.PrintString` "Trap Applied")
      (`self.ShowSelectedCard`))))

(event `/Game/FrameWork/Data/Interfaces/BPI_CardInterface.FlipCard`
  ;[0.1302 1 0] FLIP CARD LOGIC
  (`self.Rotate Card Sideways`)
  (`self.ShowSelectedCard`)
  (bind _aspc_player_controller (cast `/Game/FrameWork/Controller/PC_PlayerController` (`GameplayStatics.GetPlayerController` 0)))
  (if (`self.bCanSee`)
    (`/Game/FrameWork/Controller/PC_PlayerController.EnableButtons` _aspc_player_controller 2)
    (`/Game/FrameWork/Game/GM_GameMode.UpdateMessage` (`self.GM Game Mode`) "Info" "Click Activate button to Activate Board Selected Card")
    (else
      (`/Game/FrameWork/Controller/PC_PlayerController.EnableButtons` _aspc_player_controller 3))))

(event `/Game/FrameWork/Data/Interfaces/BPI_CardInterface.UnHighlightCard`
  (if (not (`self.bIsSelected`))
    (`PrimitiveComponent.SetRenderCustomDepth` (`self.FrontWidget`) false)
    (`PrimitiveComponent.SetRenderCustomDepth` (`self.CardMesh`) false)
    (if (`self.bCanSee`)
      _)))

(event `/Game/FrameWork/Data/Interfaces/BPI_CardInterface.HighlightCard`
  (if (not (`self.bIsSelected`))
    (`PrimitiveComponent.SetRenderCustomDepth` (`self.FrontWidget`) true)
    (`PrimitiveComponent.SetRenderCustomDepth` (`self.CardMesh`) true)))

(event `Rotate Card Forward`
  (bind (_returnvalue_roll _returnvalue_pitch _returnvalue_yaw) (`KismetMathLibrary.BreakRotator` (`SceneComponent.K2_GetComponentRotation` (`self.CardMesh`))))
  (if (`self.bIsOnBoard`)
    (if (`self.bCanSee`)
      (bind (_direction _alpha) (`Timeline|Timeline_Rotation` :!label _label_2)
        (:`Update`
          (`SceneComponent.K2_SetWorldRotation` (`self.CardMesh`) (`KismetMathLibrary.MakeRotator` _returnvalue_roll (`KismetMathLibrary.Lerp` 90.0 0.0 _alpha) _returnvalue_yaw) false false))
        (:`Finished`
          (set `self.bCanSee` (not (`self.bCanSee`)))))
      (else
        (goto _label_2 :!via `Reverse`)))))

(event `MoveTo`
  (params (Location :type "Vector Structure"))
  (bind (_direction _alpha) (`Timeline|Timeline`)
    (:`Update`
      (`self.K2_SetActorLocation` (`KismetMathLibrary.VLerp` (`self.K2_GetActorLocation`) Location _alpha))
      (`KismetSystemLibrary.PrintString` "Moving"))))

(event `self.ReceiveDestroyed`
  (`parent.ReceiveDestroyed`)
  (`KismetSystemLibrary.PrintString` "Card Destroyed in BPBase Card Graph"))

(event `Rotate Card Sideways`
  (bind (_returnvalue_roll _returnvalue_pitch _returnvalue_yaw) (`KismetMathLibrary.BreakRotator` (`SceneComponent.K2_GetComponentRotation` (`self.CardMesh`))))
  (if (`self.bIsOnBoard`)
    (if (`self.bCanSee`)
      (bind (_direction _alpha) (`Timeline|Timeline_0` :!label _label_3)
        (:`Update`
          (`SceneComponent.K2_SetWorldRotation` (`self.CardMesh`) (`KismetMathLibrary.MakeRotator` (`KismetMathLibrary.Lerp` 180.0 0.0 _alpha) _returnvalue_pitch _returnvalue_yaw) false false))
        (:`Finished`
          (set `self.bCanSee` (not (`self.bCanSee`)))))
      (else
        (goto _label_3 :!via `Reverse`)))))

(event `SetupUIHud`
  (bind _aspc_player_controller (cast `/Game/FrameWork/Controller/PC_PlayerController` (`GameplayStatics.GetPlayerController` 0)))
  (bind _ashbp_hud (cast `/Game/FrameWork/UI/HBP_HUD` (`PlayerController.GetHUD` _aspc_player_controller)))
  (bind _aswb_card_hud (cast `/Game/FrameWork/UI/Widgets/WB_CardHUD` (`/Game/FrameWork/UI/HBP_HUD.ActiveWidgetRef` _ashbp_hud)))
  (set `self.WB Card HUD UI ref` _aswb_card_hud))

(event `ShowSelectedCard`
  (bind _wb_card_hud_ui_ref (`self.WB Card HUD UI ref`))
  (bind _gm_game_mode (`self.GM Game Mode`))
  (bind _asgi_game_instance (cast `/Game/FrameWork/Game/GI_GameInstance` (`GameplayStatics.GetGameInstance`)))
  (bind _success (`/Game/FrameWork/Blueprint/Character/BP_PlayerBase.SetSelectedCard` (`/Game/FrameWork/Game/GI_GameInstance.PlayerOne` _asgi_game_instance) self))
  (if _success
    (`/Engine/EditorBlueprintResources/StandardMacros.IsValid` _wb_card_hud_ui_ref
      (:`Is Valid`
        (if (`self.bCanSee`)
          (`/Game/FrameWork/UI/Widgets/WB_CardHUD.CardSelected` _wb_card_hud_ui_ref (`self.CardInfo`))
          (if (`self.bIsOnBoard`)
            (`/Game/FrameWork/Game/GM_GameMode.UpdateMessage` _gm_game_mode "Info" "Click Activate Button to activate this cards ability")
            (else
              (`/Game/FrameWork/Game/GM_GameMode.UpdateMessage` _gm_game_mode "Info" "Select a Cell to continue")))
          (else
            (`/Game/FrameWork/UI/Widgets/WB_CardHUD.SelectedCardCancelled` _wb_card_hud_ui_ref)))))
    (else
      (`KismetSystemLibrary.PrintString` "Cannot select this card" true true (struct :`R` 0.579167 :`B` 0.021519 :`A` 1.0)))))

(fn `AddActorRef`
  (params (`Actor Ref` :type "/Game/FrameWork/Blueprint/Unit/BP_UnitBase Object Reference"))
  (returns (`Spawned Ref` :type "/Game/FrameWork/Blueprint/Unit/BP_UnitBase Object Reference"))
  (bind (_name _image _info _type _rank _unit _actorclass _actorref _backgroundcolor _attackpower _attackadd _attackmult _defencepower _defenceadd _defencemult) (break `/Game/FrameWork/Data/Struct/S_Card` (`self.CardInfo`)))
  (set `self.CardInfo` (make `/Game/FrameWork/Data/Struct/S_Card` _name _image _info _type _rank _unit null `Actor Ref` _backgroundcolor _attackpower _attackadd _attackmult _defencepower _defenceadd _defencemult))
  (bind _output_get (set `self.SpawnedUnitRef` `Actor Ref`))
  (return _output_get))

(fn `GetCardType`
  (returns (Type :type "/Game/FrameWork/Data/Enum/E_CardType Enum"))
  (return (`.Type_5_47F263B84F9A2675CF9D8B876A5B2917` (break `/Game/FrameWork/Data/Struct/S_Card` (`self.CardInfo`)))))

(fn `MoveCardToBoard`
  (locals (`Active Player` :type "/Game/FrameWork/Blueprint/Character/BP_PlayerBase Object Reference"))
  (bind _active_player (`local.Active Player`))
  (bind (_selectedcard _selectedcell) (`/Game/FrameWork/Blueprint/Character/BP_PlayerBase.GetPlayerSelectedData` _active_player))
  (bind _returnvalue (`KismetStringLibrary.Conv_NameToString` (`.Name` (`/Game/FrameWork/Blueprint/Character/BP_PlayerBase.GetPlayerInfo` _active_player))))
  (bind _asgi_game_instance (cast `/Game/FrameWork/Game/GI_GameInstance` (`GameplayStatics.GetGameInstance`)))
  (bind _asgm_game_mode (cast `/Game/FrameWork/Game/GM_GameMode` (`GameplayStatics.GetGameMode`)))
  (if (`/Game/FrameWork/Game/GM_GameMode.bIsPlayerTurn` _asgm_game_mode)
    (set `local.Active Player` (`/Game/FrameWork/Game/GI_GameInstance.PlayerOne` _asgi_game_instance))
    (else
      (set `local.Active Player` (`/Game/FrameWork/Game/GI_GameInstance.PlayerTwo` _asgi_game_instance))))
  (if (and (== self _selectedcard) (> (`/Game/FrameWork/Blueprint/Character/BP_PlayerBase.MoveCountPerTurn` _active_player) 0))
    (`self.MoveTo` (`SceneComponent.K2_GetComponentLocation` (`/Game/FrameWork/Blueprint/Grid/BP_GridCell.SpawnDirectionArrow` _selectedcell)))
    (set `/Game/FrameWork/Blueprint/Grid/BP_GridCell.bISOccupied` true _selectedcell)
    (set `self.bIsOnBoard` true)
    (`self.Rotate Card Forward`)
    (set `self.bCanSee` false)
    (`/Game/FrameWork/Blueprint/Character/BP_PlayerBase.MoveCardToBoard` _active_player)
    (`/Game/FrameWork/Game/GM_GameMode.UpdateMessage` (`self.GM Game Mode`) (`KismetTextLibrary.Conv_StringToText` (`KismetStringLibrary.Concat_StrStr` _returnvalue " Main On Info")) (`KismetTextLibrary.Conv_StringToText` (`KismetStringLibrary.Concat_StrStr` _returnvalue " can Click on Card on Board to Activate Card")))))

(fn `UserConstructionScript`)