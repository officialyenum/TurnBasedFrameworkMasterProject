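; BP_UnitBase is a unit actor Blueprint in the Card framework that reacts to cursor hover on its skeletal mesh.
; BeginPlay binds the Mesh cursor-over events: hover start prints the actor's display name, and hover end destroys OutlineMesh if it is valid.
; Nothing in these graphs creates OutlineMesh, and the construction script is empty, with an unconnected node for setting the mesh from PlayerMesh.
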(event `self.ReceiveBeginPlay`
  (bind _mesh (`self.Mesh`))
  (add `PrimitiveComponent.OnBeginCursorOver` _mesh (delegate `OnBeginCursorOver_Event`))
  (add `PrimitiveComponent.OnEndCursorOver` _mesh (delegate `OnEndCursorOver_Event`)))

(event `OnBeginCursorOver_Event`
  (params (TouchedComponent :type "PrimitiveComponent Object Reference"))
  (`KismetSystemLibrary.PrintString` (`KismetSystemLibrary.GetDisplayName` self)))

(event `OnEndCursorOver_Event`
  (params (TouchedComponent :type "PrimitiveComponent Object Reference"))
  (bind _outlinemesh (`self.OutlineMesh`))
  (`/Engine/EditorBlueprintResources/StandardMacros.IsValid` _outlinemesh
    (:`Is Valid`
      (`ActorComponent.K2_DestroyComponent` _outlinemesh))))

(fn `UserConstructionScript`)