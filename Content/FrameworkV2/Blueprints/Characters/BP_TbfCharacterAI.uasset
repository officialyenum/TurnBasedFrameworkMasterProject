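; AI-controlled character Blueprint for a game with cards and units on a board, extending a parent character's UI events.
; Its stat update calls the parent, then reaches the first player's HUD overlay through controller casts to show the AI's name and unit and card counts.
; The message event follows the same path but sends an empty string to the overlay rather than the incoming text.
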(event `self.ReceiveBeginPlay`
  (`parent.ReceiveBeginPlay`))

(event `self.ShowMessageInUI`
  (params (Text :type "Text (by ref)"))
  (`parent.ShowMessageInUI` Text)
  (bind _asbp_tbf_player_controller (cast `/Game/FrameworkV2/Blueprints/Player/BP_TbfPlayerController` (`GameplayStatics.GetPlayerController` 0)))
  (bind _asbp_tbf_hud (cast `/Game/FrameworkV2/Blueprints/UI/HUD/BP_TbfHUD` (`PlayerController.GetHUD` _asbp_tbf_player_controller)))
  (bind _aswbp_tbf_overlay (cast `/Game/FrameworkV2/Blueprints/UI/Widgets/WBP_TbfOverlay` (`TbfHUD.OverlayWidget` _asbp_tbf_hud)))
  (`/Game/FrameworkV2/Blueprints/UI/Widgets/WBP_TbfOverlay.UpdateMessage` _aswbp_tbf_overlay ""))

(event `self.UpdateUIStat`
  (`parent.UpdateUIStat`)
  (bind _asbp_tbf_player_controller (cast `/Game/FrameworkV2/Blueprints/Player/BP_TbfPlayerController` (`GameplayStatics.GetPlayerController` 0)))
  (bind _asbp_tbf_hud (cast `/Game/FrameworkV2/Blueprints/UI/HUD/BP_TbfHUD` (`PlayerController.GetHUD` _asbp_tbf_player_controller)))
  (bind _aswbp_tbf_overlay (cast `/Game/FrameworkV2/Blueprints/UI/Widgets/WBP_TbfOverlay` (`TbfHUD.OverlayWidget` _asbp_tbf_hud)))
  (`/Game/FrameworkV2/Blueprints/UI/Widgets/WBP_TbfOverlay.UpdateAIStat` _aswbp_tbf_overlay (`KismetTextLibrary.Conv_NameToText` (`self.Name`)) 0.0 (`KismetArrayLibrary.Array_Length` (`self.UnitOnField`)) (`KismetArrayLibrary.Array_Length` (`self.Hand`)) (`self.Deck`) (`KismetArrayLibrary.Array_Length` (`self.CardOnField`))))

(fn `UserConstructionScript`)