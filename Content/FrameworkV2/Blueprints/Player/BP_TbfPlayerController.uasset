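; Player controller Blueprint for the Tbf framework that toggles game pause.
; Its PauseGameEvent override calls the parent, then checks IsPaused and tells BP_TbfGameMode to resume or pause the game.
; Direct pause and resume calls to BP_TbfHUD are present but disconnected, and BeginPlay, Tick and the construction script are empty.
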(event `self.ReceiveBeginPlay`)

(event `self.PauseGameEvent`
  (bind _returnvalue (`GameplayStatics.GetGameMode`))
  (`parent.PauseGameEvent`)
  (if (`self.bIsPaused`)
    (bind _asbp_tbf_game_mode (cast `/Game/FrameworkV2/Blueprints/Game/BP_TbfGameMode` _returnvalue))
    (`TbfGameMode.ResumeGame` _asbp_tbf_game_mode)
    (else
      (bind _asbp_tbf_game_mode_2 (cast `/Game/FrameworkV2/Blueprints/Game/BP_TbfGameMode` _returnvalue))
      (`TbfGameMode.PauseGame` _asbp_tbf_game_mode_2))))

(fn `UserConstructionScript`)