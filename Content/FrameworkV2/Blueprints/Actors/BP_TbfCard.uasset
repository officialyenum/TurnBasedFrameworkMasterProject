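; BP_TbfCard is a clickable card actor that supports selection, movement and display of its card info.
; Clicking toggles selection, registering a newly selected card on the player character.
; A timeline lerps the card from its current location to a target, while setup passes CardInfo to the front widget.
; ShowCardinUI sets the card as PlayerOne's selection in the game instance and updates the HUD overlay.
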(event `self.ReceiveBeginPlay`
  (`parent.ReceiveBeginPlay`)
  (add `self.OnClicked` (delegate `OnClicked_Event`)))

(event `OnClicked_Event` :!signature `self.OnClicked`
  (params (TouchedActor :type "Actor Object Reference") (ButtonPressed :type "Key Structure" :default "None"))
  (`KismetSystemLibrary.PrintString` "Clicked")
  (if (`self.bCardIsSelected`)
    (`self.UnSelectActor`)
    (else
      (`self.SelectActor`)
      (bind _asbp_tbf_character (cast `/Game/FrameworkV2/Blueprints/Characters/BP_TbfCharacter` (`GameplayStatics.GetPlayerCharacter` 0)))
      (bind _output_get (set `TbfCharacter.SelectedCard` self _asbp_tbf_character))
      (`KismetSystemLibrary.PrintString` (`KismetStringLibrary.Concat_StrStr` "Selected " (`KismetSystemLibrary.GetDisplayName` _output_get))))))

(event `self.MoveCardToLocation`
  (params (Location :type "Vector Structure (by ref)"))
  (bind (_direction _alpha) (`Timeline|Timeline`)
    (:`Update`
      (`self.K2_SetActorLocation` (`KismetMathLibrary.VLerp` (`self.K2_GetActorLocation`) Location _alpha)))))

(event `self.SetUpCard`
  (`parent.SetUpCard`)
  (bind _aswbp_tbf_card (cast `/Game/FrameworkV2/Blueprints/UI/Widgets/WBP_TbfCard` (`WidgetComponent.GetUserWidgetObject` (`self.FrontWidget`))))
  (`/Game/FrameworkV2/Blueprints/UI/Widgets/WBP_TbfCard.UpdateCardInfo` _aswbp_tbf_card (`self.CardInfo`)))

(event `self.ShowCardInUI`
  (`parent.ShowCardInUI`)
  (bind _asbp_tbf_game_instance (cast `/Game/FrameworkV2/Blueprints/Game/BP_TbfGameInstance` (`GameplayStatics.GetGameInstance`)))
  (set `TbfCharacter.SelectedCard` self (`TbfGameInstance.PlayerOne` _asbp_tbf_game_instance))
  (bind _asbp_tbf_hud (cast `/Game/FrameworkV2/Blueprints/UI/HUD/BP_TbfHUD` (`PlayerController.GetHUD` (`GameplayStatics.GetPlayerController` 0))))
  (bind _aswbp_tbf_overlay (cast `/Game/FrameworkV2/Blueprints/UI/Widgets/WBP_TbfOverlay` (`TbfHUD.OverlayWidget` _asbp_tbf_hud)))
  (`/Game/FrameworkV2/Blueprints/UI/Widgets/WBP_TbfOverlay.CardSelected` _aswbp_tbf_overlay (`self.CardInfo`)))

(fn `UserConstructionScript`)