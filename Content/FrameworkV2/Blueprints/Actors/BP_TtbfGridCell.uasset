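; BP_TtbfGridCell is a grid cell actor that responds to mouse hover and clicks for highlighting and selection.
; BeginPlay binds the cursor events, with hover calling highlight and unhighlight functions defined outside these graphs.
; Clicking toggles selection, first asking BP_GridManager, found by GetActorOfClass, to reset the grid's selection before selecting this cell.
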(event `self.ReceiveBeginPlay`
  (add `Actor.OnBeginCursorOver` (delegate `OnBeginCursorOver_Event`))
  (add `Actor.OnEndCursorOver` (delegate `OnEndCursorOver_Event`))
  (add `Actor.OnClicked` (delegate `OnClicked_Event`)))

(event `OnBeginCursorOver_Event`
  (params (TouchedActor :type "Actor Object Reference"))
  (`self.HighlightActor`))

(event `OnEndCursorOver_Event`
  (params (TouchedActor :type "Actor Object Reference"))
  (`self.UnHighlightActor`))

(event `OnClicked_Event`
  (params (TouchedActor :type "Actor Object Reference") (ButtonPressed :type "Key Structure" :default "None"))
  (if (`self.bCellIsSelected`)
    (`self.UnSelectActor`)
    (else
      (bind _returnvalue (`GameplayStatics.GetActorOfClass` "/Game/FrameWork/Blueprint/Grid/BP_GridManager.BP_GridManager_C"))
      (`/Game/FrameWork/Blueprint/Grid/BP_GridManager.Reset Grid Selection` _returnvalue)
      (`self.SelectActor`))))

(fn `UserConstructionScript`)